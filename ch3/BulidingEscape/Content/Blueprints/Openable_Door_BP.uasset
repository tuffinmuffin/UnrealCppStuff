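; Openable door Blueprint that swings its static mesh open and closed around the yaw axis.
; Open and close request events from its OpenDoor member each restart their own timeline, OpenRate or CloseRate, from the beginning.
; Each timeline update sets the mesh's relative rotation directly, without sweep.
; Because the two timelines are separate and always play from start, neither request resumes from the door's current angle.
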(event OnOpenRequest(OpenDoor)
  (Development|PrintString "OpenEvent" false false "(R=0.205482,G=1.000000,B=0.000000,A=1.000000)")
  (bind _openangle (Timeline|OpenRate PlayFromStart)
    (:Update
      (Transformation|SetRelativeRotation (Variables|Debug|GetStaticMeshComponent) (Math|Rotator|MakeRotator 0.0 0.0 _openangle) false false))))

(event OnCloseRequest(OpenDoor)
  (Development|PrintString "CloseEvent" false false "(R=1.000000,G=0.186432,B=0.367106,A=1.000000)")
  (bind _closerate (Timeline|CloseRate PlayFromStart)
    (:Update
      (Transformation|SetRelativeRotation (Variables|Debug|GetStaticMeshComponent) (Math|Rotator|MakeRotator 0.0 0.0 _closerate) false false))))

(fn ConstructionScript)